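; VR player that lets the user gaze at, pick up and drop objects implementing BPI_VRObjects.
; An eye-ray trace each tick, while nothing is held, updates the focused actor and sends focus gained or lost calls.
; A touch tap picks up the focused actor or drops the held one.
; A timeline lerps picked objects to a set distance along the eye ray, where Tick keeps them; construction places the cursor sphere there too.
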(event Custom|OnFocusActorChanged
  (params (Actor :type Actor%20Object%20Reference))
  ;[1 1 1] Focus Actor Changed
  (if (!= Actor (Variables|Default|GetFocusActor))
    (Utilities|FlowControl|Sequence
      (:then_0
        (Utilities|IsValid (Variables|Default|GetFocusActor)
          (:Is%20Valid
            (bind _asbpi_vrobjects (Utilities|Casting|CastToBPI_VRObjects (Variables|Default|GetFocusActor)))
            (Default|LostFocus _asbpi_vrobjects))))
      (:then_1
        (bind _output_get (Variables|Default|SetFocusActor Actor))
        (Utilities|IsValid _output_get
          (:Is%20Valid
            (bind _asbpi_vrobjects_2 (Utilities|Casting|CastToBPI_VRObjects _output_get))
            (Default|OnFocus _asbpi_vrobjects_2)))))))

(event Custom|PickupFocusActor
  (bind _focusactor (Variables|Default|GetFocusActor))
  ;[1 1 1] Pickup Focus Actor
  (Utilities|FlowControl|Sequence
    (:then_0
      (bind _asbpi_vrobjects (Utilities|Casting|CastToBPI_VRObjects _focusactor))
      (Default|OnPickup _asbpi_vrobjects))
    (:then_1
      (Variables|Default|SetPickedActor _focusactor))
    (:then_2
      (bind _output_get (Variables|Default|SetPickActorInitLoc (Transformation|GetActorLocation _focusactor)))
      (Variables|Default|SetPickAnim true)
      (bind _alpha (Timeline|Timeline_0 PlayFromStart)
        (:Update
          (Transformation|SetActorLocation (Variables|Default|GetPickedActor) (Math|Vector|Lerp(Vector) _output_get (Utilities|GetLocationonEyeRay (Variables|Default|GetDisatnce)) _alpha) false false))
        (:Finished
          (Variables|Default|SetPickAnim false))))))

(event Custom|DropActor
  ;[1 1 1] Drop Actor
  (Utilities|FlowControl|Sequence
    (:then_0
      (bind _asbpi_vrobjects (Utilities|Casting|CastToBPI_VRObjects (Variables|Default|GetPickedActor)))
      (Default|OnDrop _asbpi_vrobjects))
    (:then_1
      (Variables|Default|SetPickedActor 0))))

(event EventTick
  (params (DeltaSeconds :type Float%20%28single-precision%29))
  (bind (_outlocation _outrotation) (Actor|GetActorEyesViewPoint))
  (Utilities|FlowControl|Sequence
    (:then_0
      ;[1 1 1] Line Trace
      (Utilities|IsValid (Variables|Default|GetPickedActor)
        (:Is%20Not%20Valid
          (bind (_outhit _returnvalue) (Collision|LineTraceByChannel _outlocation (|(StartLoc+(Forward*Dist)) _outlocation (Math|Vector|GetForwardVector _outrotation) 5e+03) "TraceTypeQuery1" false 0 "None"))
          (if (and _returnvalue (Utilities|DoesObjectImplementInterface (.HitActor (Collision|BreakHitResult _outhit)) "/Game/Blueprints/BPI_VRObjects.BPI_VRObjects_C"))
            (CallFunction|OnFocusActorChanged (.HitActor (Collision|BreakHitResult _outhit)))
            (else
              (CallFunction|OnFocusActorChanged))))))
    (:then_1
      (if (and (Utilities|IsValid (Variables|Default|GetPickedActor)) (not (Variables|Default|GetPickAnim)))
        (Transformation|SetActorLocation (Variables|Default|GetPickedActor) (Utilities|GetLocationonEyeRay (Variables|Default|GetDisatnce)) false false)))))

(event EventOnTouchTap
  ;[1 1 1] Touch Tap Event
  (Utilities|IsValid (Variables|Default|GetPickedActor)
    (:Is%20Valid
      (CallFunction|DropActor))
    (:Is%20Not%20Valid
      (Utilities|IsValid (Variables|Default|GetFocusActor)
        (:Is%20Valid
          (CallFunction|PickupFocusActor))))))

(fn ConstructionScript
  ;[1 1 1] Set Cursor Objects Location
  (Transformation|SetWorldLocation (Variables|Default|GetCursorShpere) (Utilities|GetLocationonEyeRay (Variables|Default|GetDisatnce)) false false))