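; BP_Block is a physics block that can be focused, picked up and dropped, showing its state through its face texture.
; Construction creates a dynamic material instance whose base color texture changes for focused, held, free awake or free sleeping states.
; Pickup turns off physics and collision, drop restores both, and rigid body wake and sleep events update the sleeping flag and texture.
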(event `/Game/Blueprints/BPI_VRObjects.OnFocus`
  ;[1 1 1] Focus Change Events
  (`MaterialInstanceDynamic.SetTextureParameterValue` (`self.BlockMaterial`) "TexBaseColor" "/Game/Textures/T_FaceC.T_FaceC"))

(event `/Game/Blueprints/BPI_VRObjects.LostFocus`
  ;[1 1 1] Focus Change Events
  (`self.ChangeTextureByState`))

(event `self.StaticMeshComponent.OnComponentWake`
  (params (WakingComponent :type "PrimitiveComponent Object Reference") (BoneName :type Name))
  ;[1 1 1] Rigid Body Events
  (set `self.IsSleeping` false)
  (`self.ChangeTextureByState` :!label _label))

(event `/Game/Blueprints/BPI_VRObjects.OnPickup`
  ;[1 1 1] Pickup & Drop
  (set `self.IsFree` false)
  (`self.ChangeTextureByState` :!label _label_2)
  (`self.EnablePhys` (`self.IsFree`)))

(event `/Game/Blueprints/BPI_VRObjects.OnDrop`
  ;[1 1 1] Pickup & Drop
  (set `self.IsFree` true)
  (goto _label_2))

(event `self.StaticMeshComponent.OnComponentSleep`
  (params (SleepingComponent :type "PrimitiveComponent Object Reference") (BoneName :type Name))
  ;[1 1 1] Rigid Body Events
  (set `self.IsSleeping` true)
  (goto _label))

(event `ChangeTextureByState`
  (bind _blockmaterial (`self.BlockMaterial`))
  ;[1 1 1] Change Texture By State
  (if (`self.IsFree`)
    (if (`self.IsSleeping`)
      (`MaterialInstanceDynamic.SetTextureParameterValue` _blockmaterial "TexBaseColor" "/Game/Textures/T_FaceB.T_FaceB")
      (else
        (`MaterialInstanceDynamic.SetTextureParameterValue` _blockmaterial "TexBaseColor" "/Game/Textures/T_FaceA.T_FaceA")))
    (else
      (`MaterialInstanceDynamic.SetTextureParameterValue` (`self.BlockMaterial`) "TexBaseColor" "/Game/Textures/T_FaceD.T_FaceD"))))

(fn `EnablePhys`
  (params (Enable :type Boolean))
  (bind _staticmeshcomponent (`self.StaticMeshComponent`))
  (`PrimitiveComponent.SetSimulatePhysics` _staticmeshcomponent Enable)
  (if Enable
    (`PrimitiveComponent.SetCollisionEnabled` _staticmeshcomponent "QueryAndPhysics")
    (else
      (`PrimitiveComponent.SetCollisionEnabled` _staticmeshcomponent "NoCollision"))))

(fn `UserConstructionScript`
  (bind _returnvalue (`PrimitiveComponent.CreateDynamicMaterialInstance` (`self.StaticMeshComponent`) 0 "/Game/Materials/M_Bloks.M_Bloks"))
  (set `self.BlockMaterial` _returnvalue))