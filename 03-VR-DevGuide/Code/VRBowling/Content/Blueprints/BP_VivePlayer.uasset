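; BP_VivePlayer is a VR player Blueprint that lets either motion controller pick up and throw bowling objects.
; Pressing a trigger snaps overlapping BP_Bowling actors to that hand's controller mesh, keeping relative rotation and scale.
; Releasing it detaches attached bowling actors, re-enables physics and collision, and copies the controller mesh's linear and angular physics velocities onto them for the throw.
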(event `Key|MotionController_Left_Trigger`
  (params (Key :type "Key Structure" :default "AnyKey"))
  (bind _mcmeshleft (`self.MCMeshLeft`))
  ;[1 1 1] Trigger Events
  (:`Pressed`
    (`self.PickupBowling` _mcmeshleft))
  (:`Released`
    (`self.Delivery` _mcmeshleft)))

(event `Key|MotionController_Right_Trigger`
  (params (Key :type "Key Structure" :default "AnyKey"))
  (bind _mcmeshright (`self.MCMeshRight`))
  ;[1 1 1] Trigger Events
  (:`Pressed`
    (`self.PickupBowling` _mcmeshright))
  (:`Released`
    (`self.Delivery` _mcmeshright)))

(event `PickupBowling`
  (params (MCMesh :type "StaticMeshComponent Object Reference"))
  ;[1 1 1] Pickup
  (for _array_element (`PrimitiveComponent.GetOverlappingActors` MCMesh "/Game/Blueprints/BP_Bowling.BP_Bowling_C")
    (`self.K2_AttachToComponent` _array_element MCMesh "None" "SnapToTarget" "KeepRelative" "KeepRelative" true)))

(event `Delivery`
  (params (MCMesh :type "StaticMeshComponent Object Reference"))
  (for _array_element (`SceneComponent.GetChildrenComponents` MCMesh false)
    (bind _asbp_bowling (cast `/Game/Blueprints/BP_Bowling` (`ActorComponent.GetOwner` _array_element)))
    (`self.K2_DetachFromActor` _asbp_bowling "KeepWorld" "KeepWorld" "KeepWorld")
    (bind _staticmeshcomponent (`StaticMeshActor.StaticMeshComponent` _asbp_bowling))
    (`PrimitiveComponent.SetSimulatePhysics` _staticmeshcomponent true)
    (`PrimitiveComponent.SetCollisionEnabled` _staticmeshcomponent "QueryAndPhysics")
    (bind _returnvalue (`PrimitiveComponent.GetPhysicsLinearVelocity` MCMesh "None"))
    (bind _returnvalue_2 (`PrimitiveComponent.GetPhysicsAngularVelocity` MCMesh "None"))
    (`PrimitiveComponent.SetPhysicsAngularVelocity` _staticmeshcomponent _returnvalue_2 false "None")
    (`PrimitiveComponent.SetPhysicsLinearVelocity` _staticmeshcomponent _returnvalue false "None")))

(fn `UserConstructionScript`)